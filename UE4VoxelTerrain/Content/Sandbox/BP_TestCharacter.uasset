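; Sandbox test player character that adds the inventory HUD on BeginPlay and maps hard-coded keys to player controller actions.
; Keys select inventory slots, pick up objects and kill the character, while UE4VoxelTerrainPlayerController handles tool and construction mode toggles.
; Tab flip-flops the full inventory, and E opens or closes a container alongside it.
; Both block game input while shown and close widgets by class lookup instead of stored references.
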(event EventBeginPlay
  (bind _returnvalue (UserInterface|CreateWidget "/Game/Sandbox/UI/WBP_PlayerInventory.WBP_PlayerInventory_C"))
  (UserInterface|Viewport|AddtoViewport _returnvalue 0))

(event Collision|EventActorBeginOverlap
  (params (OtherActor :type Actor%20Object%20Reference)))

(event EventTick
  (params (DeltaSeconds :type Float%20%28single-precision%29)))

(event Input|KeyboardEvents|Tab
  (params (Key :type Key%20Structure :default "None"))
  (:Pressed
    (bind _assandbox_player_controller (Utilities|Casting|CastToSandboxPlayerController (Game|GetPlayerController 0)))
    (Utilities|FlowControl|FlipFlop
      (:A
        (Class|SandboxPlayerController|BlockGameInput _assandbox_player_controller)
        (bind _returnvalue (UserInterface|CreateWidget "/Game/Sandbox/UI/WBP_PlayerInventoryFull.WBP_PlayerInventoryFull_C"))
        (UserInterface|Viewport|AddtoViewport _returnvalue 0))
      (:B
        (Class|SandboxPlayerController|UnblockGameInput _assandbox_player_controller)
        (bind _foundwidgets (Widget|GetAllWidgetsOfClass "/Game/Sandbox/UI/WBP_PlayerInventoryFull.WBP_PlayerInventoryFull_C" true))
        (Widget|RemovefromParent _foundwidgets)))))

(event Input|KeyboardEvents|R
  (params (Key :type Key%20Structure :default "None"))
  (:Pressed
    (bind _assandbox_player_controller (Utilities|Casting|CastToSandboxPlayerController (Game|GetPlayerController 0)))
    (Class|SandboxPlayerController|TakeObjecttoInventory _assandbox_player_controller)))

(event Input|KeyboardEvents|T
  (params (Key :type Key%20Structure :default "None"))
  (:Pressed
    (bind _asue4voxel_terrain_player_controller (Utilities|Casting|CastToUE4VoxelTerrainPlayerController (Game|GetPlayerController 0)))
    (Class|UE4VoxelTerrainPlayerController|ToggleConstructionMode _asue4voxel_terrain_player_controller)))

(event Input|KeyboardEvents|E
  (params (Key :type Key%20Structure :default "None"))
  (:Pressed
    (bind _assandbox_player_controller (Utilities|Casting|CastToSandboxPlayerController (Game|GetPlayerController 0)))
    (bind _returnvalue (Class|SandboxPlayerController|HasOpenContainer _assandbox_player_controller))
    (if _returnvalue
      (Class|SandboxPlayerController|CloseObjectwithContainer _assandbox_player_controller)
      (bind _foundwidgets (Widget|GetAllWidgetsOfClass "/Game/Sandbox/UI/WBP_PlayerOpenContainer.WBP_PlayerOpenContainer_C" true))
      (Widget|RemovefromParent _foundwidgets)
      (bind _foundwidgets_2 (Widget|GetAllWidgetsOfClass "/Game/Sandbox/UI/WBP_PlayerInventoryFull.WBP_PlayerInventoryFull_C" true))
      (Widget|RemovefromParent _foundwidgets_2)
      (Class|SandboxPlayerController|UnblockGameInput _assandbox_player_controller)
      (else
        (bind _returnvalue_2 (Class|SandboxPlayerController|OpenObjectwithContainer _assandbox_player_controller))
        (if _returnvalue_2
          (bind _returnvalue_3 (UserInterface|CreateWidget "/Game/Sandbox/UI/WBP_PlayerOpenContainer.WBP_PlayerOpenContainer_C"))
          (UserInterface|Viewport|AddtoViewport _returnvalue_3 0)
          (bind _returnvalue_4 (UserInterface|CreateWidget "/Game/Sandbox/UI/WBP_PlayerInventoryFull.WBP_PlayerInventoryFull_C"))
          (UserInterface|Viewport|AddtoViewport _returnvalue_4 0)
          (Class|SandboxPlayerController|BlockGameInput _assandbox_player_controller))))))

(event Input|KeyboardEvents|F
  (params (Key :type Key%20Structure :default "None"))
  (:Pressed
    (bind _asue4voxel_terrain_player_controller (Utilities|Casting|CastToUE4VoxelTerrainPlayerController (Game|GetPlayerController 0)))
    (Class|UE4VoxelTerrainPlayerController|ToggleToolMode _asue4voxel_terrain_player_controller)))

(event Input|KeyboardEvents|P
  (params (Key :type Key%20Structure :default "None"))
  (:Pressed
    (Utilities|Casting|CastToSandboxPlayerController (Game|GetPlayerController 0))
    (Class|SandboxCharacter|Kill)))

(event Input|KeyboardEvents|1
  (params (Key :type Key%20Structure :default "None"))
  (:Pressed
    (bind _assandbox_player_controller (Utilities|Casting|CastToSandboxPlayerController (Game|GetPlayerController 0)))
    (Class|SandboxPlayerController|SetCurrentInventoryslot _assandbox_player_controller)))

(event Input|KeyboardEvents|2
  (params (Key :type Key%20Structure :default "None"))
  (:Pressed
    (bind _assandbox_player_controller (Utilities|Casting|CastToSandboxPlayerController (Game|GetPlayerController 0)))
    (Class|SandboxPlayerController|SetCurrentInventoryslot _assandbox_player_controller 1)))

(event Input|KeyboardEvents|3
  (params (Key :type Key%20Structure :default "None"))
  (:Pressed
    (bind _assandbox_player_controller (Utilities|Casting|CastToSandboxPlayerController (Game|GetPlayerController 0)))
    (Class|SandboxPlayerController|SetCurrentInventoryslot _assandbox_player_controller 2)))

(fn ConstructionScript)